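; BP_MainHero is the player-controlled hero, with movement, look and pointer interaction with widgets.
; BeginPlay adds the IMC_Main Enhanced Input context, whose move and look actions drive movement along the actor's axes and controller yaw and inverted pitch.
; The left mouse action presses or releases the pointer key on a WidgetInteraction component, whose hover-change event stores the current WidgetComponent.
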(event OnHoveredWidgetChanged(WidgetInteraction)
  (params (WidgetComponent :type Widget%20Component%20Object%20Reference) (PreviousWidgetComponent :type Widget%20Component%20Object%20Reference))
  ;[0.15 0.15 0.15 0.5] This Event Trigger the same as Hover/Unhover
  (Variables|Default|SetWidget%20Component WidgetComponent))

(event Input|EnhancedActionEvents|EnhancedInputActionIA_Move
  (params (ActionValue :type Vector%202D%20Structure) (ElapsedSeconds :type Float%20%28double-precision%29) (TriggeredSeconds :type Float%20%28double-precision%29) (InputAction :type Input%20Action%20Object%20Reference :default "/Game/Inputs/IA_Move.IA_Move"))
  (:Triggered
    (Pawn|Input|AddMovementInput (+ (* (.x ActionValue) (Transformation|GetActorForwardVector)) (* (.y ActionValue) (Transformation|GetActorRightVector))) 1.0 false)))

(event Input|EnhancedActionEvents|EnhancedInputActionIA_Look
  (params (ActionValue :type Vector%202D%20Structure) (ElapsedSeconds :type Float%20%28double-precision%29) (TriggeredSeconds :type Float%20%28double-precision%29) (InputAction :type Input%20Action%20Object%20Reference :default "/Game/Inputs/IA_Look.IA_Look"))
  (:Triggered
    (Pawn|Input|AddControllerPitchInput (* (.y ActionValue) -1.0))
    (Pawn|Input|AddControllerYawInput (.x ActionValue))))

(event Input|EnhancedActionEvents|EnhancedInputActionIA_MouseLeftBtn
  (params (ActionValue :type Boolean) (ElapsedSeconds :type Float%20%28double-precision%29) (TriggeredSeconds :type Float%20%28double-precision%29) (InputAction :type Input%20Action%20Object%20Reference :default "/Game/Inputs/IA_MouseLeftBtn.IA_MouseLeftBtn"))
  (bind _widgetinteraction (Variables|Default|GetWidgetInteraction))
  (:Triggered
    (if ActionValue
      (Utilities|IsValid _widgetinteraction
        (:Is%20Valid
          (Class|WidgetInteractionComponent|PressPointerKey _widgetinteraction "LeftMouseButton")))
      (else
        (Utilities|IsValid _widgetinteraction
          (:Is%20Valid
            (Class|WidgetInteractionComponent|ReleasePointerKey _widgetinteraction "LeftMouseButton")))))))

(event EventBeginPlay
  (Input|AddMappingContext (PlayerController|LocalPlayerSubsystems|GetEnhancedInputLocalPlayerSubsystem (Game|GetPlayerController 0)) "/Game/Inputs/IMC_Main.IMC_Main" 0 "(bIgnoreAllPressedKeysUntilRelease=True,bForceImmediately=False,bNotifyUserSettings=False)"))

(event Collision|EventActorBeginOverlap
  (params (OtherActor :type Actor%20Object%20Reference)))

(event EventTick
  (params (DeltaSeconds :type Float%20%28single-precision%29)))

(fn ConstructionScript)